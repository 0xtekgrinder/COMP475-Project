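; Hand component that records and recognises static hand gestures from bone poses, for left or right hands.
; Recording stores component-space bone locations under a unique name in a BP_SG_Gesture save slot, with deletion by name; DeleteAllGestures is unfinished.
; A looping timer compares live bones against gestures loaded at BeginPlay, taking the first with every bone within Threshold.
; Each tick broadcasts an update, and matches broadcast current and previous gesture names.
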(event Custom|DetectGesture
  (Default|CallOnGestureUpdate (Variables|Default|GetDetectRate))
  (bind (_detected _gesture) (CallFunction|GetCurrentGesture))
  (if _detected
    (Variables|Default|SetLastGesture (Variables|Default|GetCurrentGesture))
    (Variables|Default|SetCurrentGesture _gesture)
    (Development|PrintString "Detected Gesture")
    (Development|PrintString (.GestureName (Utilities|Struct|BreakS_Gesture (Variables|Default|GetCurrentGesture))))
    (Default|CallOnGestureRecognised (.GestureName (Utilities|Struct|BreakS_Gesture (Variables|Default|GetCurrentGesture))) (Variables|Default|GetMeshType) self (.GestureName (Utilities|Struct|BreakS_Gesture (Variables|Default|GetLastGesture))))))

(event EventBeginPlay
  (Variables|Default|SetGestures (Variables|/Game/Hands/BP_SG_Gesture.BP_SG_Gesture_C|GetGestures (CallFunction|LoadGesture)))
  (Utilities|Time|SetTimerbyEvent (delegate Custom|DetectGesture) (Variables|Default|GetDetectRate) true))

(fn RecordGesture
  (params (GestureName :type String))
  (bind _output_get (LocalVariables|SetSG_Gestures (CallFunction|LoadGesture)))
  (if (not (CallFunction|DoesGestureExist? _output_get GestureName))
    (for _index (range 0 (- (Class|SkinnedMeshComponent|GetNumBones) 1))
      (bind _returnvalue (Class|PoseableMeshComponent|GetBoneLocationbyName (Class|SkinnedMeshComponent|GetBoneName _index) "ComponentSpace"))
      (Utilities|Array|Add (LocalVariables|GetBoneLocations) _returnvalue))
    (Utilities|Array|Add (Variables|/Game/Hands/BP_SG_Gesture.BP_SG_Gesture_C|GetGestures (LocalVariables|GetSG_Gestures)) (Utilities|Struct|MakeS_Gesture GestureName (LocalVariables|GetBoneLocations)))
    (SaveGame|SaveGametoSlot (LocalVariables|GetSG_Gestures) (Variables|Default|GetGestureGameSlot))
    (Development|PrintString "Saved new gesture in slot")
    (Development|PrintString GestureName)))

(fn DoesGestureExist?
  (params (SG_Gestures :type BP%20SG%20Gesture%20Object%20Reference) (GestureName :type String))
  (for _array_element (Variables|/Game/Hands/BP_SG_Gesture.BP_SG_Gesture_C|GetGestures SG_Gestures)
    (if (Utilities|Enum|Equal(Enum) (.GestureName (Utilities|Struct|BreakS_Gesture _array_element)) GestureName)
      (return true)))
  (return false))

(fn LoadGesture
  (if (Utilities|Enum|Equal(Enum) (Variables|Default|GetMeshType) "HandLeft")
    (Development|PrintString "Loading gesture for Left hand"))
  (bind _returnvalue (SaveGame|DoesSaveGameExist (Variables|Default|GetGestureGameSlot)))
  (if _returnvalue
    (bind _returnvalue_2 (SaveGame|LoadGamefromSlot (Variables|Default|GetGestureGameSlot)))
    (bind _asbp_sg_gesture (Utilities|Casting|CastToBP_SG_Gesture _returnvalue_2))
    (if (Utilities|Enum|Equal(Enum) (Variables|Default|GetMeshType) "HandLeft")
      (Development|PrintString "LOADED SAVE"))
    (return _asbp_sg_gesture)
    (else
      (bind _returnvalue_3 (SaveGame|CreateSaveGameObject "/Game/Hands/BP_SG_Gesture.BP_SG_Gesture_C"))
      (return _returnvalue_3))))

(fn DeleteGesturebyName
  (params (GestureName :type String))
  (bind _output_get (LocalVariables|SetGestures (CallFunction|LoadGesture)))
  (for (_array_element _array_index) (Variables|/Game/Hands/BP_SG_Gesture.BP_SG_Gesture_C|GetGestures _output_get)
    (if (Utilities|Enum|Equal(Enum) (.GestureName (Utilities|Struct|BreakS_Gesture _array_element)) GestureName)
      (LocalVariables|SetindexToDelete _array_index)))
  (Utilities|Array|RemoveIndex (Variables|/Game/Hands/BP_SG_Gesture.BP_SG_Gesture_C|GetGestures (LocalVariables|GetGestures)) (LocalVariables|GetindexToDelete))
  (SaveGame|SaveGametoSlot (LocalVariables|GetGestures) (Variables|Default|GetGestureGameSlot)))

(fn DeleteAllGestures
  (bind _output_get (LocalVariables|SetNewLocalVar (CallFunction|LoadGesture))))

(fn GetCurrentGesture
  (for _array_element (Variables|Default|GetGestures)
    (for (_array_element_2 _array_index) (.BonesLocation (Utilities|Struct|BreakS_Gesture _array_element))
      (bind _returnvalue (Class|PoseableMeshComponent|GetBoneLocationbyName (Class|SkinnedMeshComponent|GetBoneName _array_index) "ComponentSpace"))
      (if (Variables|Default|GetDebug)
        (Development|PrintString (Utilities|String|Append "Abs of gesture: " (Utilities|String|ToString(Float) (Math|Float|Absolute(Float) (Math|Vector|VectorLength (- _returnvalue _array_element_2)))))))
      (if (> (Math|Float|Absolute(Float) (Math|Vector|VectorLength (- _returnvalue _array_element_2))) (Variables|Default|GetThreshold))
        (LocalVariables|SetbValidGesture? false)))
    (if (LocalVariables|GetbValidGesture?)
      (return true _array_element)
      (else
        (LocalVariables|SetbValidGesture? true))))
  (return false ""))

(fn EqualGesture
  (params (A :type S%20Gesture%20Structure) (B :type S%20Gesture%20Structure))
  (bind (_gesturename _boneslocation) (Utilities|Struct|BreakS_Gesture A))
  (bind (_gesturename_2 _boneslocation_2) (Utilities|Struct|BreakS_Gesture B))
  (return (and (Utilities|Enum|Equal(Enum) _gesturename _gesturename_2) (Utilities|Array|Identical _boneslocation _boneslocation_2))))